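; BP_timesquence drives the day-night cycle from CurrentTime stored in the GIS game instance.
; Tick advances that clock faster than real time and converts it to a day fraction that sets the directional light's pitch.
; Clamped range maps raise light intensity and tint directional and sky lights toward white each morning, without an evening ramp down.
; Nested color lerps shift height fog through night, day, sunset and back to night.
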(event `self.ReceiveBeginPlay`
  ; 게임을 시작할때 GIS(게임 인스턴스 설정해놓은거)로부터 시간을 받는다
  (bind _asgis (cast `/Game/BluePrints/GIS` (`GameplayStatics.GetGameInstance`)))
  (set `self.mygis` _asgis))

(event `self.ReceiveTick`
  (params (DeltaSeconds :type "Float (single-precision)"))
  (bind _timepercent (`self.timepercent`))
  (bind _daynight (`self.Daynight`))
  (bind _lightcomponent (`Light.LightComponent` _daynight))
  (bind _returnvalue (`KismetMathLibrary.LinearColorLerp` (struct :`G` 0.200615 :`B` 0.25 :`A` 1.0) (struct :`R` 1.0 :`G` 1.0 :`B` 1.0 :`A` 1.0) (`KismetMathLibrary.MapRangeClamped` _timepercent 0.2 0.25 0.0 1.0)))
  ; event tick 이용하여 시간의 흐름 이용 delta seconds 연결된 multiply 노드에서 배율 정해서 현실 시간보다 빠르게 정함 지금 디폴트 기준은 60초 빠르게 흘러감
  (bind _output_get (set `/Game/BluePrints/GIS.current_time` (+ (`/Game/BluePrints/GIS.current_time` (`self.mygis`)) (`KismetMathLibrary.FromSeconds` (* DeltaSeconds 60.0))) (`self.mygis`)))
  (bind (_year _month _day _hour _minute) (`KismetMathLibrary.BreakDateTime` _output_get))
  ; directional light  pitch 계산을 위한 계산식들
  (bind _output_get_2 (set `self.timepercent` (/ (`KismetMathLibrary.Conv_IntToDouble` (+ (* _hour 60) _minute)) 1440.0)))
  (`self.K2_SetActorRotation` _daynight (`KismetMathLibrary.MakeRotator` 0.0 (`KismetMathLibrary.Conv_IntToDouble` (+ (* _output_get_2 360.0) 90))) false)
  ; directional light 강도 조절, 낮일때 6, 밤일때 0.05로 조정
  (`LightComponent.SetIntensity` _lightcomponent (`KismetMathLibrary.MapRangeClamped` _timepercent 0.2 0.5 0.05 6.0))
  ; fog 색 변경 관련 노드
  (`ExponentialHeightFogComponent.SetFogInscatteringColor` (`ExponentialHeightFog.Component` (`self.Exponenetial HEight fog`)) (`KismetMathLibrary.LinearColorLerp` (`KismetMathLibrary.LinearColorLerp` (`KismetMathLibrary.LinearColorLerp` (struct :`R` 0.000911 :`G` 0.001214 :`B` 0.017642 :`A` 1.0) (struct :`R` 1.0 :`G` 1.0 :`B` 1.0 :`A` 1.0) (`KismetMathLibrary.MapRangeClamped` _timepercent 0.2 0.3 0.0 1.0)) (struct :`R` 0.817708 :`G` 0.218535 :`B` 0.030748 :`A` 1.0) (`KismetMathLibrary.MapRangeClamped` _timepercent 0.7 0.75 0.0 1.0)) (struct :`R` 0.000911 :`G` 0.001214 :`B` 0.016807 :`A` 1.0) (`KismetMathLibrary.MapRangeClamped` _timepercent 0.76 0.78 0.0 1.0)))
  ; 왼쪽은 directional light 쪽, 오른쪽은 밤에 스카이 라이트 조정 (왼쪽은 삭제 해도 무방할것임)
  (`LightComponent.SetLightColor` _lightcomponent _returnvalue false)
  (`SkyLightComponent.SetLightColor` (`SkyLight.LightComponent` (`self.skylight`)) _returnvalue))

(fn `UserConstructionScript`)